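; Wind spell actor, apparently the third Q spell, that travels along world X and knocks characters into the air.
; On BeginPlay, the WindSpawn timeline adds its Travel value to the X location each update and sets a uniform scale from ScaleWind.
; When its mesh overlaps a BP_ThirdPersonCharacter, it adds that character to the player character's ListofBumped and launches it straight upward.
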(event `self.ReceiveBeginPlay`
  (bind (_returnvalue_x _returnvalue_y _returnvalue_z) (`KismetMathLibrary.BreakVector` (`self.K2_GetActorLocation`)))
  (bind (_direction _scalewind _travel) (`Timeline|WindSpawn`)
    (:`Update`
      (`self.K2_SetActorLocation` (`KismetMathLibrary.MakeVector` (+ _returnvalue_x _travel) _returnvalue_y _returnvalue_z))
      (`self.SetActorScale3D` (`KismetMathLibrary.Conv_DoubleToVector` _scalewind)))))

(event `self.StaticMesh.OnComponentBeginOverlap`
  (params (OverlappedComponent :type "PrimitiveComponent Object Reference") (OtherActor :type "Actor Object Reference") (OtherComp :type "PrimitiveComponent Object Reference") (OtherBodyIndex :type Integer) (bFromSweep :type Boolean) (SweepResult :type "HitResult Structure (by ref)"))
  (bind _asbp_third_person_character (cast `/Game/ThirdPerson/Blueprints/BP_ThirdPersonCharacter` OtherActor))
  (bind _asbp_player_character (cast `/Game/GameBank/Blueprints/Characters/BP_PlayerCharacter` (`GameplayStatics.GetPlayerCharacter` 0)))
  (`KismetArrayLibrary.Array_Add` (`/Game/GameBank/Blueprints/Characters/BP_PlayerCharacter.ListofBumped` _asbp_player_character) _asbp_third_person_character)
  (`Character.LaunchCharacter` _asbp_third_person_character (0.0 0.0 750.0) false false))

(fn `UserConstructionScript`)