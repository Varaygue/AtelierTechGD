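; Player character modeled on Yasuo, with Enhanced Input movement, montage-driven sword attacks, HUD and sword-trace damage helper.
; Q cycles three montages on a timeline cooldown, or while dashing enables a sphere that destroys overlapped characters; E dashes via timeline lerp.
; R teleports to the first bumped actor and plays the ultimate.
; Tick polls for the third-Q tornado spawn and ultimate camera blend, both behind never-reset DoOnce nodes.
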(event `self.ReceiveTick`
  (params (DeltaSeconds :type "Float (single-precision)"))
  (`|ExecutionSequence`
    (:`then_0`
      (if (== (`self.qSpellCount`) 3)
        (`/Engine/EditorBlueprintResources/StandardMacros.DoOnce` false
          (:`Completed`
            (`|SpawnActorFromClass` "/Game/GameBank/Blueprints/Ingredients/BP_qSpell3.BP_qSpell3_C" (`KismetMathLibrary.MakeTransform` (`SceneComponent.K2_GetComponentLocation` (`self.TornadoSpawn`)) (`self.GetControlRotation` (`GameplayStatics.GetPlayerCharacter` 0))) "Undefined" "MultiplyWithRoot" null null)))))
    (:`then_1`
      (`KismetSystemLibrary.PrintString` (`KismetStringLibrary.Conv_IntToString` (`KismetArrayLibrary.Array_Length` (`self.ListofBumped`)))))
    (:`then_2`
      (`/Engine/EditorBlueprintResources/StandardMacros.Gate` true :!label _label
        (:`Exit`
          (`/Engine/EditorBlueprintResources/StandardMacros.DoOnce` false
            (:`Completed`
              (`PlayerController.SetViewTargetWithBlend` (`GameplayStatics.GetPlayerController` 0) (`ChildActorComponent.ChildActor` (`self.ChildActor`)) 0.2 "VTBlend_Linear" 0.0 false)
              (`KismetSystemLibrary.Delay` 1.0)
              (`PlayerController.SetViewTargetWithBlend` (`GameplayStatics.GetPlayerController` 0) (`GameplayStatics.GetPlayerCharacter` 0) 0.2 "VTBlend_Linear" 0.0 false))))))))

(event `DoTransition`
  (goto _label :!via `Open`))

(event `self.ReceiveBeginPlay`
  (bind _returnvalue (`GameplayStatics.GetPlayerCameraManager` 0))
  (`EnhancedInputSubsystemInterface.AddMappingContext` (pcsubsystem `EnhancedInputLocalPlayerSubsystem` (`GameplayStatics.GetPlayerController` 0)) "/Game/GameBank/Blueprints/Characters/IMC_PlayerInputs.IMC_PlayerInputs" 0 (struct))
  (bind _returnvalue_2 (`|CreateWidget` "/Game/GameBank/HUD/WBP_PlayerHUD.WBP_PlayerHUD_C"))
  (bind _output_get (set `self.PlayerHUD` _returnvalue_2))
  (`UserWidget.AddToViewport` _output_get 0)
  (set `PlayerCameraManager.ViewPitchMin` -30.0 _returnvalue)
  (set `PlayerCameraManager.ViewPitchMax` 30.0 _returnvalue)
  (`KismetArrayLibrary.Array_Clear` (`self.ListofBumped`)))

(event `EnhancedInput|/Game/GameBank/Blueprints/Characters/IA_MovingRight`
  (params (ActionValue :type "Float (double-precision)") (ElapsedSeconds :type "Float (double-precision)") (TriggeredSeconds :type "Float (double-precision)") (InputAction :type "InputAction Object Reference" :default "/Game/GameBank/Blueprints/Characters/IA_MovingRight.IA_MovingRight"))
  (bind (_returnvalue_roll _returnvalue_pitch _returnvalue_yaw) (`KismetMathLibrary.BreakRotator` (`self.GetControlRotation`)))
  (:`Triggered`
    (`self.AddMovementInput` (`KismetMathLibrary.GetRightVector` (`KismetMathLibrary.MakeRotator` _returnvalue_roll 0.0 _returnvalue_yaw)) ActionValue)))

(event `EnhancedInput|/Game/GameBank/Blueprints/Characters/IA_MovingForward`
  (params (ActionValue :type "Float (double-precision)") (ElapsedSeconds :type "Float (double-precision)") (TriggeredSeconds :type "Float (double-precision)") (InputAction :type "InputAction Object Reference" :default "/Game/GameBank/Blueprints/Characters/IA_MovingForward.IA_MovingForward"))
  (bind (_returnvalue_roll _returnvalue_pitch _returnvalue_yaw) (`KismetMathLibrary.BreakRotator` (`self.GetControlRotation`)))
  (:`Triggered`
    (`self.AddMovementInput` (`KismetMathLibrary.GetForwardVector` (`KismetMathLibrary.MakeRotator` 0.0 0.0 _returnvalue_yaw)) ActionValue)))

(event `EnhancedInput|/Game/GameBank/Blueprints/Characters/IA_CameraLook`
  (params (ActionValue :type "Vector2D Structure") (ElapsedSeconds :type "Float (double-precision)") (TriggeredSeconds :type "Float (double-precision)") (InputAction :type "InputAction Object Reference" :default "/Game/GameBank/Blueprints/Characters/IA_CameraLook.IA_CameraLook"))
  (:`Triggered`
    (`self.AddControllerYawInput` ActionValue_X)
    (`self.AddControllerPitchInput` ActionValue_Y)))

(event `Key|E`
  (params (Key :type "Key Structure"))
  (:`Pressed`
    (`self.DashBegin`)
    (`/Game/GameBank/HUD/WBP_PlayerHUD.Espell` (`self.PlayerHUD`))))

(event `DashBegin`
  (set `self.Dashing?` true)
  (`|PlayMontage` (`self.Mesh`) "/Game/GameBank/Character/AM_YasuoDashh.AM_YasuoDashh" (/ 1.06 (`self.DashDuration`) 2.0)
    (:`then`
      (`self.MoveOverTime` (+ (`self.K2_GetActorLocation`) (* (`self.GetActorForwardVector`) 800.0)))
      (`KismetSystemLibrary.Delay` 1.0)
      (set `self.Dashing?` false))))

(event `MoveOverTime`
  (params (Location :type "Vector Structure"))
  (bind _output_get (set `self.DashStartLocation` (`self.K2_GetActorLocation`)))
  (`self.K2_SetActorRotation` (`KismetMathLibrary.FindLookAtRotation` _output_get Location))
  (`TimelineComponent.SetPlayRate` (`self.DashTimeline`) (/ 1.0 (`self.DashDuration`)))
  (bind (_direction _locationtrack) (`Timeline|DashTimeline` :!via `PlayFromStart`)
    (:`Update`
      (`self.K2_SetActorLocation` (`KismetMathLibrary.VLerp` (`self.DashStartLocation`) Location _locationtrack) false true))))

(event `EnhancedInput|/Game/GameBank/Blueprints/Characters/IA_Attack`
  (params (ActionValue :type Boolean) (ElapsedSeconds :type "Float (double-precision)") (TriggeredSeconds :type "Float (double-precision)") (InputAction :type "InputAction Object Reference" :default "/Game/GameBank/Blueprints/Characters/IA_Attack.IA_Attack"))
  (:`Triggered`
    (if (not (`self.Attacking?`))
      (`self.FaceCameraDirection`)
      (set `self.swordOut` true)
      (set `self.Attacking?` true)
      (`|PlayMontage` (`self.Mesh`) (select `int` (`self.AttackCount`) :`0` "/Game/GameBank/Character/AM_YasuoAttack.AM_YasuoAttack" :`1` "/Game/Characters/AM_YasuoAttack02.AM_YasuoAttack02" :!type "AnimMontage Object Reference")
        (:`then`
          (`/Engine/EditorBlueprintResources/StandardMacros.IncrementInt` (`self.AttackCount`)))
        (:`OnCompleted`
          (set `self.AttackCount` 0 :!label _label_2))
        (:`OnInterrupted`
          (`KismetSystemLibrary.RetriggerableDelay` 1.0)
          (set `self.Attacking?` false)
          (goto _label_2))))))

(event `EnhancedInput|/Game/GameBank/Blueprints/Characters/IA_Qspell`
  (params (ActionValue :type Boolean) (ElapsedSeconds :type "Float (double-precision)") (TriggeredSeconds :type "Float (double-precision)") (InputAction :type "InputAction Object Reference" :default "/Game/GameBank/Blueprints/Characters/IA_Qspell.IA_Qspell"))
  (bind _mesh (`self.Mesh`))
  (bind _qspellcount (`self.qSpellCount`))
  (bind _sphere (`self.Sphere`))
  (:`Triggered`
    (if (`self.Spell1Up`)
      (`self.FaceCameraDirection`)
      (set `self.swordOut` true)
      (set `self.Spell1Up` false)
      (`CharacterMovementComponent.SetMovementMode` (`self.CharacterMovement`) "MOVE_None" 0)
      (if (not (`self.Dashing?`))
        (`|PlayMontage` _mesh (select `int` (`self.qSpellCount`) :`0` "/Game/GameBank/Character/AM_YasuoQspell1.AM_YasuoQspell1" :`1` "/Game/GameBank/Character/qSpell2/AM_YasuoqSpell2.AM_YasuoqSpell2" :`2` "/Game/GameBank/Character/qSpell3/AM_YasuoqSpell3.AM_YasuoqSpell3" :!type "AnimMontage Object Reference")
          (:`then`
            (bind (_direction _newtrack_0) (`Timeline|spellCooldown` :!via `PlayFromStart` :!label _label_3)
              (:`Update`
                (set `self.Spell1Cooldown` _newtrack_0))
              (:`Finished`
                (set `self.Spell1Up` true)
                (`/Engine/EditorBlueprintResources/StandardMacros.IncrementInt` _qspellcount
                  (:`  `
                    (if (== _qspellcount 3)
                      (`KismetSystemLibrary.Delay` 0.2)
                      (set `self.qSpellCount` 0)))))))
          (:`OnNotifyBegin`
            (`CharacterMovementComponent.SetMovementMode` (`self.CharacterMovement`) "MOVE_Walking" 0)))
        (else
          (set `PrimitiveComponent.bGenerateOverlapEvents` true _sphere)
          (`|PlayMontage` _mesh "/Game/GameBank/Character/Qspelldash/AM_YasuoQspelldash.AM_YasuoQspelldash"
            (:`then`
              (goto _label_3 :!via `PlayFromStart`))
            (:`OnNotifyBegin`
              (set `PrimitiveComponent.bGenerateOverlapEvents` false _sphere)
              (`CharacterMovementComponent.SetMovementMode` (`self.CharacterMovement`) "MOVE_Walking" 0))))))))

(event `self.Sphere.OnComponentBeginOverlap`
  (params (OverlappedComponent :type "PrimitiveComponent Object Reference") (OtherActor :type "Actor Object Reference") (OtherComp :type "PrimitiveComponent Object Reference") (OtherBodyIndex :type Integer) (bFromSweep :type Boolean) (SweepResult :type "HitResult Structure (by ref)"))
  (bind _asbp_third_person_character (cast `/Game/ThirdPerson/Blueprints/BP_ThirdPersonCharacter` OtherActor))
  (`self.K2_DestroyActor` _asbp_third_person_character))

(event `SheatingSword`
  (set `self.swordOut` false))

(event `Key|R`
  (params (Key :type "Key Structure"))
  (bind _listofbumped (`self.ListofBumped`))
  (bind (_returnvalue_x _returnvalue_y) (`KismetMathLibrary.BreakVector` (`self.K2_GetActorLocation` (`|GetArrayItem` _listofbumped))))
  (:`Released`
    (if (`KismetArrayLibrary.Array_IsNotEmpty` _listofbumped)
      (`self.K2_SetActorLocation` (`KismetMathLibrary.MakeVector` _returnvalue_x _returnvalue_y))
      (`|PlayMontage` (`self.Mesh`) "/Game/GameBank/Character/Ult/AM_YasuoUlt.AM_YasuoUlt"
        (:`then`
          (`self.DoTransition`))))))

(fn `FaceCameraDirection`
  (`self.K2_SetActorRotation` (`self.GetControlRotation` (`GameplayStatics.GetPlayerCharacter` 0))))

(fn `HitDetect`
  (bind _returnvalue (`SceneComponent.GetSocketLocation` (`self.Mesh`) "SwordBlade3"))
  (bind (_outhit _returnvalue_2) (`KismetSystemLibrary.SphereTraceSingleForObjects` :`Start` _returnvalue :`End` _returnvalue :`Radius` 50.0 :`ObjectTypes` (`|MakeArray` "ObjectTypeQuery3" :!type "EObjectTypeQuery Enum") :`DrawDebugType` "ForDuration" :`DrawTime` 1.0))
  (if _returnvalue_2
    (bind _asbp_third_person_character (cast `/Game/ThirdPerson/Blueprints/BP_ThirdPersonCharacter` (`.HitActor` (`GameplayStatics.BreakHitResult` _outhit))))
    (`GameplayStatics.ApplyDamage` _asbp_third_person_character 50.0)))

(fn `UltCameraTransition`
  (params (DeltaSeconds :type "Float (double-precision)"))
  (`SceneComponent.K2_SetWorldLocation` (`self.Camera`) (`KismetMathLibrary.VInterpTo` (`SceneComponent.K2_GetComponentLocation` (`self.Camera`)) (`SplineComponent.FindLocationClosestToWorldLocation` (`self.Spline`) (`self.K2_GetActorLocation`) "World") DeltaSeconds 2.0) false false))

(fn `UserConstructionScript`)