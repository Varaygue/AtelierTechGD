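; BP_LunedoCharacter is a side-scrolling player character that moves along the Y axis, jumps and toggles a grab on the BP_Jarre jar.
; Enhanced Input moves it left or right, interpolates mesh facing and sets direction flags.
; Tick caches delta time and resets location keeping only Y and Z, locking the movement plane.
; Grab line-traces along the mesh's right vector; a hit enables the jar's physics, and releasing disables it.
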(event `self.ReceiveTick`
  (params (DeltaSeconds :type "Float (single-precision)"))
  (bind (_returnvalue_x _returnvalue_y _returnvalue_z) (`KismetMathLibrary.BreakVector` (`self.K2_GetActorLocation`)))
  (set `self.Delta Seconds` DeltaSeconds)
  (`self.K2_SetActorLocation` (`KismetMathLibrary.MakeVector` 0.0 _returnvalue_y _returnvalue_z)))

(event `self.ReceiveBeginPlay`
  (`EnhancedInputSubsystemInterface.AddMappingContext` (pcsubsystem `EnhancedInputLocalPlayerSubsystem` (`GameplayStatics.GetPlayerController` 0)) "/Game/LuneDo/GameBank/Inputs/IMC_LunedoInputs.IMC_LunedoInputs" 0 (struct))
  (bind _returnvalue (`GameplayStatics.GetActorOfClass` "/Game/LuneDo/GameBank/Blueprints/Ingrédients/BP_Jarre.BP_Jarre_C"))
  (set `self.JarreRef` _returnvalue))

(event `EnhancedInput|/Game/LuneDo/GameBank/Inputs/InputAction_MoveLeft`
  (params (ActionValue :type Boolean) (ElapsedSeconds :type "Float (double-precision)") (TriggeredSeconds :type "Float (double-precision)") (InputAction :type "InputAction Object Reference" :default "/Game/LuneDo/GameBank/Inputs/InputAction_MoveLeft.InputAction_MoveLeft"))
  (:`Triggered`
    (`self.AddMovementInput` (0.0 -1.0 0.0))
    (`SceneComponent.K2_SetWorldRotation` (`self.Mesh`) (`KismetMathLibrary.RInterpTo` (`SceneComponent.K2_GetComponentRotation` (`self.Mesh`)) (struct :`Yaw` 180.0) (`self.Delta Seconds`) 10.0) false false)
    (set `self.Left` true)
    (set `self.Right` false)))

(event `EnhancedInput|/Game/LuneDo/GameBank/Inputs/InputAction_MoveRight`
  (params (ActionValue :type Boolean) (ElapsedSeconds :type "Float (double-precision)") (TriggeredSeconds :type "Float (double-precision)") (InputAction :type "InputAction Object Reference" :default "/Game/LuneDo/GameBank/Inputs/InputAction_MoveRight.InputAction_MoveRight"))
  (:`Triggered`
    (`self.AddMovementInput` (0.0 1.0 0.0))
    (`SceneComponent.K2_SetWorldRotation` (`self.Mesh`) (`KismetMathLibrary.RInterpTo` (`SceneComponent.K2_GetComponentRotation` (`self.Mesh`)) (struct) (`self.Delta Seconds`) 10.0) false false)
    (set `self.Right` true)
    (set `self.Left` false)))

(event `EnhancedInput|/Game/LuneDo/GameBank/Inputs/InputAction_Jump`
  (params (ActionValue :type Boolean) (ElapsedSeconds :type "Float (double-precision)") (TriggeredSeconds :type "Float (double-precision)") (InputAction :type "InputAction Object Reference" :default "/Game/LuneDo/GameBank/Inputs/InputAction_Jump.InputAction_Jump"))
  (:`Triggered`
    (`self.Jump`)))

(event `EnhancedInput|/Game/LuneDo/GameBank/Inputs/InputAction_Grab`
  (params (ActionValue :type Boolean) (ElapsedSeconds :type "Float (double-precision)") (TriggeredSeconds :type "Float (double-precision)") (InputAction :type "InputAction Object Reference" :default "/Game/LuneDo/GameBank/Inputs/InputAction_Grab.InputAction_Grab"))
  (bind _mesh (`self.Mesh`))
  (bind _returnvalue (`SceneComponent.K2_GetComponentLocation` _mesh))
  (:`Triggered`
    (if (`self.isGrabbing`)
      (set `self.isGrabbing` false)
      (`PrimitiveComponent.SetSimulatePhysics` (`/Game/LuneDo/GameBank/Blueprints/Ingrédients/BP_Jarre.Jarre` (`self.JarreRef`)) false)
      (else
        (bind _outhit (`KismetSystemLibrary.LineTraceSingle` :`Start` (+ _returnvalue (0.0 0.0 75.0)) :`End` (+ (+ _returnvalue (* (`SceneComponent.GetRightVector` _mesh) 100.0)) (0.0 0.0 75.0)) :`TraceChannel` "TraceTypeQuery3" :`TraceColor` (struct :`R` 1.0 :`G` 0.865307 :`A` 1.0) :`DrawTime` 0.0))
        (if (`GameplayStatics.BreakHitResult` _outhit)
          (set `self.isGrabbing` true)
          (`PrimitiveComponent.SetSimulatePhysics` (`/Game/LuneDo/GameBank/Blueprints/Ingrédients/BP_Jarre.Jarre` (`self.JarreRef`)) true))))))

(fn `UserConstructionScript`)